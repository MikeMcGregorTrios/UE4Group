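; GunFP_BP is a first-person gun that arms when the TopDownCharacter switches to first-person view.
; Tick polls that switch, running a once-only delayed activation that shows Aim, enables shooting and later disables mesh shadows, and reversing this on exit.
; While armed, holding left mouse spawns BULLET_BP, an emitter and a shot sound at the Arrow, with a Delay in Tick throttling the fire rate.
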(event `self.ReceiveBeginPlay`
  (`SceneComponent.SetVisibility` (`self.Aim`) false false))

(event `Activate_FirstPerson`
  (`KismetSystemLibrary.Delay` 6.0)
  (`SceneComponent.SetVisibility` (`self.Aim`) true false)
  (set `self.Activation_Shooting` true)
  (`KismetSystemLibrary.Delay` 2.0)
  (`PrimitiveComponent.SetCastShadow` (`self.ACWR_MAG`) false)
  (`PrimitiveComponent.SetCastShadow` (`self.ACWR_Mesh_0004`) false)
  (`PrimitiveComponent.SetCastShadow` (`self.ACWR_Mesh_0005`) false)
  (`PrimitiveComponent.SetCastShadow` (`self.ACWR_Mesh_0006`) false)
  (`PrimitiveComponent.SetCastShadow` (`self.ACWR_Mesh_0007`) false)
  (`PrimitiveComponent.SetCastShadow` (`self.ACWR_TRIGGER`) false)
  (`PrimitiveComponent.SetCastShadow` (`self.ACWR_BOLT`) false))

(event `self.ReceiveTick`
  (params (DeltaSeconds :type "Float (single-precision)"))
  (bind _arrow (`self.Arrow`))
  (bind _returnvalue (`SceneComponent.K2_GetComponentLocation` _arrow))
  (bind _astop_down_character (cast `/Game/TopDownBP/Blueprints/TopDownCharacter` (`GameplayStatics.GetPlayerCharacter` 0)))
  (if (`/Game/TopDownBP/Blueprints/TopDownCharacter.Switch_To_First_Person` _astop_down_character)
    (`|ExecutionSequence`
      (:`then_0`
        (`/Engine/EditorBlueprintResources/StandardMacros.DoOnce` false :!label _label
          (:`Completed`
            (`self.Activate_FirstPerson`))))
      (:`then_1`
        (if (and (`PlayerController.IsInputKeyDown` (`GameplayStatics.GetPlayerController` 0) "LeftMouseButton") (`self.Activation_Shooting`))
          (`KismetSystemLibrary.Delay` 0.1)
          (`|SpawnActorFromClass` "/Game/FPWeapon/BULLET_BP.BULLET_BP_C" (`SceneComponent.K2_GetComponentToWorld` _arrow) "Undefined" "OverrideRootScale" null null)
          (`GameplayStatics.SpawnEmitterAtLocation` null _returnvalue (struct) (0.05 0.05 0.05))
          (`GameplayStatics.SpawnSoundAtLocation` "/Game/FPWeapon/Single_Shot_Cue.Single_Shot_Cue" _returnvalue (struct) 1.0 1.0 0.0 null null)
          (`KismetSystemLibrary.PrintString` "Shooting"))))
    (else
      (`SceneComponent.SetVisibility` (`self.Aim`) false false)
      (`PrimitiveComponent.SetCastShadow` (`self.ACWR_MAG`) true)
      (`PrimitiveComponent.SetCastShadow` (`self.ACWR_Mesh_0004`) true)
      (`PrimitiveComponent.SetCastShadow` (`self.ACWR_Mesh_0005`) true)
      (`PrimitiveComponent.SetCastShadow` (`self.ACWR_Mesh_0006`) true)
      (`PrimitiveComponent.SetCastShadow` (`self.ACWR_Mesh_0007`) true)
      (`PrimitiveComponent.SetCastShadow` (`self.ACWR_TRIGGER`) true)
      (`PrimitiveComponent.SetCastShadow` (`self.ACWR_BOLT`) true)
      (set `self.Activation_Shooting` false)
      (goto _label :!via `Reset`))))

(fn `UserConstructionScript`)